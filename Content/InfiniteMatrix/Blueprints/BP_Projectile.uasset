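; BP_Projectile is a player-scoring projectile that destroys enemies on contact in the InfiniteMatrix game.
; Each tick it looks up the first BP_Player and sweeps along world X at that player's forward speed plus a fixed offset.
; Overlapping a BP_Enemy adds points to the player's score, then destroys both the projectile and the enemy.
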(event `self.ReceiveTick`
  (params (DeltaSeconds :type "Float (single-precision)"))
  (bind _outactors (`GameplayStatics.GetAllActorsOfClass` "/Game/InfiniteMatrix/Blueprints/BP_Player.BP_Player_C"))
  (bind _output_get (set `self.PlayerReference` (`|GetArrayItem` _outactors)))
  (`self.K2_AddActorWorldOffset` (`KismetMathLibrary.MakeVector` (* DeltaSeconds (+ (`/Game/InfiniteMatrix/Blueprints/BP_Player.ForwardSpeed` _output_get) 2000.0))) true))

(event `self.Projectile.OnComponentBeginOverlap`
  (params (OverlappedComponent :type "PrimitiveComponent Object Reference") (OtherActor :type "Actor Object Reference") (OtherComp :type "PrimitiveComponent Object Reference") (OtherBodyIndex :type Integer) (bFromSweep :type Boolean) (SweepResult :type "HitResult Structure (by ref)"))
  (bind _playerreference (`self.PlayerReference`))
  (bind _asbp_enemy (cast `/Game/InfiniteMatrix/Blueprints/BP_Enemy` OtherActor))
  (set `/Game/InfiniteMatrix/Blueprints/BP_Player.Score` (+ (`/Game/InfiniteMatrix/Blueprints/BP_Player.Score` _playerreference) 3) _playerreference)
  (`self.K2_DestroyActor`)
  (`self.K2_DestroyActor` _asbp_enemy))

(fn `UserConstructionScript`)